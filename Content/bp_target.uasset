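; Target actor that generates a screenshot dataset with 2D bounding-box labels for its Shahed mesh.
; A looping timer teleports the player pawn around the target, aims it with random in-FOV offsets, and waits briefly.
; It projects eight oriented-bounds corners to screen, appends their min/max at 1080p scale to a CSV, and has bp_cameraPawn take an indexed screenshot.
; The debug box and movement nodes are disconnected.
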(event `self.ReceiveBeginPlay`
  (set `self.screenshotIndex` 0)
  (`KismetSystemLibrary.K2_SetTimerDelegate` (delegate `event`) 2.0 true true))

(event `self.ReceiveTick`
  (params (DeltaSeconds :type "Float (single-precision)")))

(event `event`
  (`self.MoveCameraViewRandomly`)
  (`KismetSystemLibrary.Delay` 1.0)
  (`self.WriteBoundingCoordinatesToAFile` (`self.shahed`) "Z:\\unreal_projekty\\data\\labels.csv" (stale _output_get))
  (bind _output_get (set `self.screenshotIndex` (+ (stale _output_get) 1))))

(fn `DrawBoundingBox`
  (params (mesh :type "StaticMeshComponent Object Reference"))
  (locals (`Transformed Points` :type "Array of Vector Structure"))
  (bind (_min _max) (`StaticMeshComponent.GetLocalBounds` mesh))
  (bind _returnvalue (`KismetMathLibrary.Vector_GetAbs` (- _max _min)))
  (`KismetSystemLibrary.DrawDebugBox` (`KismetMathLibrary.MakeVector` (.x (`SceneComponent.K2_GetComponentLocation` mesh)) (.y (`SceneComponent.K2_GetComponentLocation` mesh)) (+ (/ (.z _returnvalue) 2.0) (.z (`SceneComponent.K2_GetComponentLocation` mesh)))) (* (/ _returnvalue 2.0) (`SceneComponent.K2_GetComponentScale` mesh)) (struct :`R` 1.0 :`G` 0.034388 :`B` 0.551621 :`A` 1.0) (`SceneComponent.K2_GetComponentRotation` mesh) 2.0 1.0))

(fn `Get Vector Permutations`
  (params (vec :type "Vector Structure"))
  (returns (`Vector Permutations` :type "Array of Vector Structure"))
  (locals (`Permutations Array` :type "Array of Vector Structure"))
  (bind _x (.x vec))
  (bind _y (.y vec))
  (bind _z (.z vec))
  (bind _permutations_array (`local.Permutations Array`))
  (bind _returnvalue (* _z -1.0))
  (bind _returnvalue_2 (* _x -1.0))
  (bind _returnvalue_3 (* _y -1.0))
  (`KismetArrayLibrary.Array_Add` _permutations_array (`KismetMathLibrary.MakeVector` _x _y _z))
  (`KismetArrayLibrary.Array_Add` _permutations_array (`KismetMathLibrary.MakeVector` _x _y _returnvalue))
  (`KismetArrayLibrary.Array_Add` _permutations_array (`KismetMathLibrary.MakeVector` _x _returnvalue_3 _z))
  (`KismetArrayLibrary.Array_Add` _permutations_array (`KismetMathLibrary.MakeVector` _x _returnvalue_3 _returnvalue))
  (`KismetArrayLibrary.Array_Add` _permutations_array (`KismetMathLibrary.MakeVector` _returnvalue_2 _returnvalue_3 _z))
  (`KismetArrayLibrary.Array_Add` _permutations_array (`KismetMathLibrary.MakeVector` _returnvalue_2 _returnvalue_3 _returnvalue))
  (`KismetArrayLibrary.Array_Add` _permutations_array (`KismetMathLibrary.MakeVector` _returnvalue_2 _y _z))
  (`KismetArrayLibrary.Array_Add` _permutations_array (`KismetMathLibrary.MakeVector` _returnvalue_2 _y _returnvalue))
  (return _permutations_array))

(fn `GetBoundingPoints`
  (params (mesh :type "StaticMeshComponent Object Reference"))
  (returns (boundingPoints :type "Array of Vector Structure"))
  (locals (`Transformed Points` :type "Array of Vector Structure"))
  (bind (_min _max) (`StaticMeshComponent.GetLocalBounds` mesh))
  (bind _transformed_points (`local.Transformed Points`))
  (bind _returnvalue (`KismetMathLibrary.Vector_GetAbs` (- _max _min)))
  (`|ExecutionSequence`
    (:`then_0`
      (bind _vector_permutations (`self.Get Vector Permutations` (* (/ _returnvalue 2.0) (`SceneComponent.K2_GetComponentScale` mesh)))))
    (:`then_1`
      (for _array_element _vector_permutations
        (`KismetArrayLibrary.Array_Add` _transformed_points (+ (`KismetMathLibrary.TransformLocation` (`KismetMathLibrary.Conv_RotatorToTransform` (`SceneComponent.K2_GetComponentRotation` mesh)) _array_element) (`KismetMathLibrary.MakeVector` (.x (`SceneComponent.K2_GetComponentLocation` mesh)) (.y (`SceneComponent.K2_GetComponentLocation` mesh)) (+ (/ (.z _returnvalue) 2.0) (.z (`SceneComponent.K2_GetComponentLocation` mesh)))))))
      (return _transformed_points))))

(fn `MoveCameraViewRandomly`
  (bind _returnvalue (`KismetMathLibrary.GetPI`))
  (bind _returnvalue_2 (`GameplayStatics.GetPlayerPawn` 0))
  (bind _returnvalue_3 (`self.K2_GetActorLocation` self))
  (bind _returnvalue_4 (`PlayerCameraManager.GetFOVAngle` (`GameplayStatics.GetPlayerCameraManager` 0)))
  (bind (_x _y) (`KismetMathLibrary.BreakVector2D` (`WidgetLayoutLibrary.GetViewportSize`)))
  (bind _returnvalue_5 (+ (* (`KismetMathLibrary.RandomUnitVector`) (`KismetMathLibrary.RandomFloatInRange` 1000.0 3000.0)) _returnvalue_3))
  (bind _returnvalue_6 (/ _returnvalue_4 2.0))
  (bind _returnvalue_7 (/ (* (`KismetMathLibrary.Atan` (/ (`KismetMathLibrary.Tan` (* _returnvalue_4 (/ _returnvalue 360.0))) (/ _x _y))) (/ 360.0 _returnvalue)) 2.0))
  (`self.K2_SetActorLocationAndRotation` _returnvalue_2 _returnvalue_5 (`KismetMathLibrary.FindLookAtRotation` _returnvalue_5 _returnvalue_3) false true)
  (`self.K2_AddActorLocalRotation` _returnvalue_2 (`KismetMathLibrary.MakeRotator` 0.0 (`KismetMathLibrary.RandomFloatInRange` (* _returnvalue_7 -1.0) _returnvalue_7) (`KismetMathLibrary.RandomFloatInRange` (* _returnvalue_6 -1.0) _returnvalue_6)) false true))

(fn `UserConstructionScript`)

(fn `WriteBoundingCoordinatesToAFile`
  (params (TargetMesh :type "StaticMeshComponent Object Reference") (FilePath :type String) (screenshotIndex :type Integer))
  (locals (CombinedString :type "Array of String") (ProjectedPoints :type "Array of Vector2D Structure") (minX :type "Float (double-precision)") (minY :type "Float (double-precision)") (maxX :type "Float (double-precision)") (maxY :type "Float (double-precision)") (finalString :type String))
  (bind _projectedpoints (`local.ProjectedPoints`))
  (bind (_x _y) (`KismetMathLibrary.BreakVector2D` (`WidgetLayoutLibrary.GetViewportSize`)))
  (bind _returnvalue (/ 1920.0 _x))
  (bind _returnvalue_2 (/ 1080.0 _y))
  (set `local.minX` 9999999999.0)
  (set `local.maxX` -99999999999.0)
  (set `local.minY` 9999999999.0)
  (set `local.maxY` -99999999999.0)
  (bind _boundingpoints (`self.GetBoundingPoints` TargetMesh))
  (for _array_element _boundingpoints
    (`KismetArrayLibrary.Array_Add` _projectedpoints (`GameplayStatics.ProjectWorldToScreen` (`GameplayStatics.GetPlayerController` 0) _array_element true)))
  (for _array_element_2 _projectedpoints
    (`|ExecutionSequence`
      (:`then_0`
        (bind (_x_2 _y_2) (`KismetMathLibrary.BreakVector2D` _array_element_2))
        (if (< _x_2 (stale _output_get))
          (bind _output_get (set `local.minX` _x_2))))
      (:`then_1`
        (if (< (stale _output_get_2) _x_2)
          (bind _output_get_2 (set `local.maxX` _x_2))))
      (:`then_2`
        (if (< _y_2 (stale _output_get_3))
          (bind _output_get_3 (set `local.minY` _y_2))))
      (:`then_3`
        (if (< (stale _output_get_4) _y_2)
          (bind _output_get_4 (set `local.maxY` _y_2))))))
  (`FileSDKBPLibrary.WriteStringToFile` FilePath (`KismetStringLibrary.Concat_StrStr` "" (`KismetStringLibrary.Conv_DoubleToString` (* _output_get _returnvalue)) ";" (`KismetStringLibrary.Conv_DoubleToString` (* _output_get_2 _returnvalue)) ";" (`KismetStringLibrary.Conv_DoubleToString` (* _output_get_3 _returnvalue_2)) ";" (`KismetStringLibrary.Conv_DoubleToString` (* _output_get_4 _returnvalue_2)) " \n") true)
  (bind _asbp_camera_pawn (cast `/Game/bp_cameraPawn` (`GameplayStatics.GetPlayerPawn` 0))
    (:`then`
      (`/Game/bp_cameraPawn.TakeAScreenshot` _asbp_camera_pawn screenshotIndex))
    (:`CastFailed`
      (`KismetSystemLibrary.PrintString` "DOJEBAL SE CAST"))))